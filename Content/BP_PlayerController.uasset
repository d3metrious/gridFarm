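; Player controller that spawns a BP_Camera on BeginPlay, makes it the view target and drives it as a free-moving demo camera.
; Key presses open and close gates that a per-tick event passes through to move and rotate the camera's spring arm.
; WASD pans horizontally, Q/E yaw, middle-mouse drag orbits with clamped pitch, and the mouse wheel zooms by changing arm length within limits.
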(event Custom|EventCameraTick
  (bind (_deltax _deltay) (Class|PlayerController|GetInputMouseDelta))
  (bind _camerarotationspeed (Variables|Default|GetCameraRotationSpeed))
  (bind _cameramovespeed (Variables|Default|GetCameraMoveSpeed))
  (bind _cameramovespeed_2 (Variables|Default|GetCameraMoveSpeed))
  (bind _democamera (Variables|Default|GetDemoCamera))
  (bind _democamera_2 (Variables|Default|GetDemoCamera))
  (bind _democamera_3 (Variables|Default|GetDemoCamera))
  (bind _springarm (Variables|/Game/BP_Camera.BP_Camera_C|GetSpringArm _democamera))
  (bind _springarm_2 (Variables|/Game/BP_Camera.BP_Camera_C|GetSpringArm _democamera_2))
  (bind _springarm_3 (Variables|/Game/BP_Camera.BP_Camera_C|GetSpringArm _democamera_3))
  (bind _returnvalue (Math|Vector|GetForwardVector _springarm_3))
  (bind _returnvalue_2 (Math|Vector|GetRightVector _springarm_3))
  (bind _relativerotation (Variables|/Script/Engine.SceneComponent|GetRelativeRotation _springarm_2))
  (bind (_roll _pitch _yaw) (Math|Rotator|BreakRotator _relativerotation))
  (bind _returnvalue_3 (Class|KismetMathLibrary|VectorNormal2D _returnvalue 0.0001))
  (Utilities|FlowControl|Sequence
    (:then_0
      ;[0 0.2956 0.7448 0.1 16] Camera Rotation
      (Utilities|FlowControl|Sequence
        (:then_0
          (Utilities|FlowControl|Gate true
            (:Exit
              (Transformation|AddRelativeRotation _springarm (Math|Rotator|MakeRotator 0.0 0.0 _camerarotationspeed) false false))))
        (:then_1
          (Utilities|FlowControl|Gate true
            (:Exit
              (Transformation|AddRelativeRotation _springarm (Math|Rotator|MakeRotator 0.0 0.0 (* _camerarotationspeed -1.0)) false false))))))
    (:then_1
      (Utilities|FlowControl|Gate true
        (:Exit
          (Transformation|SetRelativeRotation _springarm_2 (Math|Rotator|MakeRotator _roll (Math|Float|ClampAngle (+ _pitch (* _deltay 4.0)) -85.0 85.0) (+ _yaw (* _deltax 4.0))) false false))))
    (:then_2
      ;[0 0.2956 0.7448 0.1 16] Camera Movement
      (Utilities|FlowControl|Sequence
        (:then_0
          (Utilities|FlowControl|Gate true
            (:Exit
              (Transformation|AddWorldOffset _springarm_3 (* _returnvalue_3 _cameramovespeed_2) false false))))
        (:then_1
          (Utilities|FlowControl|Gate true
            (:Exit
              (Transformation|AddWorldOffset _springarm_3 (* _returnvalue_3 (* _cameramovespeed_2 -1.0)) false false))))
        (:then_2
          (Utilities|FlowControl|Gate true
            (:Exit
              (Transformation|AddWorldOffset _springarm_3 (* _returnvalue_2 (* _cameramovespeed -1.0)) false false))))
        (:then_3
          (Utilities|FlowControl|Gate true
            (:Exit
              (Transformation|AddWorldOffset _springarm_3 (* _returnvalue_2 _cameramovespeed) false false))))))))

(event EventBeginPlay
  (bind _returnvalue (Game|SpawnActorfromClass "/Game/BP_Camera.BP_Camera_C" (Math|Transform|MakeTransform "0, 0, 0" "0, 0, 0" "1.000000,1.000000,1.000000") "Undefined" 0 0))
  (bind _output_get (Variables|Default|SetDemoCamera _returnvalue))
  (Game|Player|SetViewTargetwithBlend _output_get 0.0 "VTBlend_Linear" 0.0 false))

(event EventTick
  (params (DeltaSeconds :type Float%20%28single-precision%29))
  (CallFunction|EventCameraTick))

(event Input|MouseEvents|MouseWheelAxis
  (params (AxisValue :type Float%20%28single-precision%29))
  (bind _democamera (Variables|Default|GetDemoCamera))
  (bind _springarm (Variables|/Game/BP_Camera.BP_Camera_C|GetSpringArm _democamera))
  ;[0 0.2956 0.7448 0.1 16] Camera Zoom
  (if (Utilities|IsValid _springarm)
    (Variables|/Script/Engine.SpringArmComponent|SetTargetArmLength (Variables|/Game/BP_Camera.BP_Camera_C|GetSpringArm (Variables|Default|GetDemoCamera)) (Math|Float|Clamp(Float) (+ (Variables|/Script/Engine.SpringArmComponent|GetTargetArmLength _springarm) (* AxisValue (Variables|Default|GetCameraZoomSpeed) -1.0)) (Variables|Default|GetCameraMinZoom) (Variables|Default|GetCameraMaxZoom)))))

(event Input|KeyboardEvents|Q
  (params (Key :type Key%20Structure))
  ;[0 0.2956 0.7448 0.1 16] Camera Rotation
  (:Pressed
    (Utilities|FlowControl|Gate true) ; enters at Open
  )
  (:Released
    (Utilities|FlowControl|Gate true) ; enters at Close
  ))

(event Input|KeyboardEvents|E
  (params (Key :type Key%20Structure))
  ;[0 0.2956 0.7448 0.1 16] Camera Rotation
  (:Pressed
    (Utilities|FlowControl|Gate true) ; enters at Open
  )
  (:Released
    (Utilities|FlowControl|Gate true) ; enters at Close
  ))

(event Input|KeyboardEvents|W
  (params (Key :type Key%20Structure))
  (bind _democamera (Variables|Default|GetDemoCamera))
  (bind _springarm (Variables|/Game/BP_Camera.BP_Camera_C|GetSpringArm _democamera))
  ;[0 0.2956 0.7448 0.1 16] Camera Movement
  (:Pressed
    (Utilities|FlowControl|Gate true) ; enters at Open
  )
  (:Released
    (Utilities|FlowControl|Gate true) ; enters at Close
  ))

(event Input|KeyboardEvents|D
  (params (Key :type Key%20Structure))
  (bind _democamera (Variables|Default|GetDemoCamera))
  (bind _springarm (Variables|/Game/BP_Camera.BP_Camera_C|GetSpringArm _democamera))
  ;[0 0.2956 0.7448 0.1 16] Camera Movement
  (:Pressed
    (Utilities|FlowControl|Gate true) ; enters at Open
  )
  (:Released
    (Utilities|FlowControl|Gate true) ; enters at Close
  ))

(event Input|KeyboardEvents|A
  (params (Key :type Key%20Structure))
  (bind _democamera (Variables|Default|GetDemoCamera))
  (bind _springarm (Variables|/Game/BP_Camera.BP_Camera_C|GetSpringArm _democamera))
  ;[0 0.2956 0.7448 0.1 16] Camera Movement
  (:Pressed
    (Utilities|FlowControl|Gate true) ; enters at Open
  )
  (:Released
    (Utilities|FlowControl|Gate true) ; enters at Close
  ))

(event Input|KeyboardEvents|S
  (params (Key :type Key%20Structure))
  (bind _democamera (Variables|Default|GetDemoCamera))
  (bind _springarm (Variables|/Game/BP_Camera.BP_Camera_C|GetSpringArm _democamera))
  ;[0 0.2956 0.7448 0.1 16] Camera Movement
  (:Pressed
    (Utilities|FlowControl|Gate true) ; enters at Open
  )
  (:Released
    (Utilities|FlowControl|Gate true) ; enters at Close
  ))

(event Input|MouseEvents|MiddleMouseButton
  (params (Key :type Key%20Structure))
  (bind (_deltax _deltay) (Class|PlayerController|GetInputMouseDelta))
  (bind _democamera (Variables|Default|GetDemoCamera))
  (bind _springarm (Variables|/Game/BP_Camera.BP_Camera_C|GetSpringArm _democamera))
  (bind _relativerotation (Variables|/Script/Engine.SceneComponent|GetRelativeRotation _springarm))
  (bind (_roll _pitch _yaw) (Math|Rotator|BreakRotator _relativerotation))
  ;[0 0.2956 0.7448 0.1 16] Camera Rotation
  (:Pressed
    (Utilities|FlowControl|Gate true) ; enters at Open
  )
  (:Released
    (Utilities|FlowControl|Gate true) ; enters at Close
  ))

(fn ConstructionScript)